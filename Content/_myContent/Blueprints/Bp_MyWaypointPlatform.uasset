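; Moving platform actor that travels through an array of waypoint actors, with a configurable mesh, speed and optional looping.
; BeginPlay hides the waypoints and starts the platform, which can also be triggered through Start.
; A timeline, its play rate set by Speed, lerps the actor's relative location between the current and next waypoint world positions.
; At each timeline event it advances the segment, or jumps back to the first when looping.
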(event `self.ReceiveBeginPlay`
  (for _array_element (`self.WayPoints`)
    (`self.SetActorHiddenInGame` _array_element true)
    (`self.PlatformStart`)))

(event `PlatformStart`
  (bind _motion_timeline (`self.Motion timeline`))
  (`self.SetFirstWaypoint`)
  (`TimelineComponent.SetPlayRate` _motion_timeline (`self.Speed`))
  (`TimelineComponent.PlayFromStart` _motion_timeline))

(fn `PathIsFinished`
  (returns (IsFinished :type Boolean))
  (return (== (`self.NextWaypointIndex`) (- (`KismetArrayLibrary.Array_Length` (`self.WayPoints`)) 1))))

(fn `Set Postions`
  (bind _waypoints (`self.WayPoints`))
  (set `self.CurrentWaypointPos` (`self.K2_GetActorLocation` (`|GetArrayItem` _waypoints (`self.CurrentWaypointIndex`))))
  (set `self.NextWaypointPos` (`self.K2_GetActorLocation` (`|GetArrayItem` _waypoints (`self.NextWaypointIndex`)))))

(fn `SetFirstWaypoint`
  (set `self.CurrentWaypointIndex` 0)
  (set `self.NextWaypointIndex` 1)
  (`self.Set Postions`))

(fn `SetNextWaypoint`
  (bind _result (`/Engine/EditorBlueprintResources/StandardMacros.IncrementInt` (`self.CurrentWaypointIndex`))
    (:`  `
      (set `self.NextWaypointIndex` (+ _result 1))
      (`self.Set Postions`))))

(fn `Start`
  (`self.PlatformStart`))

(fn `UserConstructionScript`
  (`StaticMeshComponent.SetStaticMesh` (`self.Platform mesh`) (`self.StaticMesh`)))