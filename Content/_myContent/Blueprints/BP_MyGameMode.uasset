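; Game mode Blueprint that locates the level's game manager and provides setup for the game's UI.
; BeginPlay caches the first BP_MyGameManager actor it finds.
; CreateUI, not called within this file, creates the abandon, win, lose, health and gold-cube count widgets, stores each reference on the manager and adds them all to the viewport.
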(event `self.ReceiveBeginPlay`
  (bind _outactors (`GameplayStatics.GetAllActorsOfClass` "/Game/_myContent/Blueprints/BP_MyGameManager.BP_MyGameManager_C"))
  (set `self.My game manager` (`|GetArrayItem` _outactors)))

(fn `CreateUI`
  (bind _my_game_manager (`/Game/_myContent/Blueprints/BP_MyFunctionLibrary.GetMyGameManager`))
  (bind _returnvalue (`|CreateWidget` "/Game/_myContent/UI/Widget_Adandon.Widget_Adandon_C"))
  (bind _output_get (set `/Game/_myContent/Blueprints/BP_MyGameManager.WidgetAbadnon` _returnvalue _my_game_manager))
  (`UserWidget.AddToViewport` _output_get 0)
  (bind _returnvalue_2 (`|CreateWidget` "/Game/_myContent/UI/Widget_Win.Widget_Win_C"))
  (bind _output_get_2 (set `/Game/_myContent/Blueprints/BP_MyGameManager.Widget_Win` _returnvalue_2 _my_game_manager))
  (`UserWidget.AddToViewport` _output_get_2 0)
  (bind _returnvalue_3 (`|CreateWidget` "/Game/_myContent/UI/Widget_Lose.Widget_Lose_C"))
  (bind _output_get_3 (set `/Game/_myContent/Blueprints/BP_MyGameManager.Widget_Lose` _returnvalue_3 _my_game_manager))
  (`UserWidget.AddToViewport` _output_get_3 0)
  (bind _returnvalue_4 (`|CreateWidget` "/Game/_myContent/UI/Widget_Health.Widget_Health_C"))
  (bind _output_get_4 (set `/Game/_myContent/Blueprints/BP_MyGameManager.Widget_Health` _returnvalue_4 _my_game_manager))
  (`UserWidget.AddToViewport` _output_get_4 0)
  (bind _returnvalue_5 (`|CreateWidget` "/Game/_myContent/UI/Widget_GoldCubesCollected.Widget_GoldCubesCollected_C"))
  (bind _output_get_5 (set `/Game/_myContent/Blueprints/BP_MyGameManager.Widget_Text1` _returnvalue_5 _my_game_manager))
  (`UserWidget.AddToViewport` _output_get_5 0))

(fn `UserConstructionScript`)