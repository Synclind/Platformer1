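; Spline platform actor that applies a configurable static mesh in its construction script and starts a motion timeline on BeginPlay through the PlatformStart event.
; Logic to place the mesh along the spline, scaling the timeline's SplineDistance by spline length, exists but is unconnected, so the platform never moves.
; That unconnected logic also passes a local-space spline location to SetWorldLocation.
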(event `self.ReceiveBeginPlay`
  (`self.Platform Start`))

(event `Platform Start`
  (bind (_direction _splinedistance) (`Timeline|MotionTimeline` :!via `PlayFromStart`)))

(fn `UserConstructionScript`
  (`StaticMeshComponent.SetStaticMesh` (`self.Platform mesh`) (`self.StaticMesh`)))